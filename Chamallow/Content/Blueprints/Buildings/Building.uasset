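; Building actor that follows the mouse cursor during placement until a left click fixes it in position.
; On BeginPlay it enables input from the first player controller and shows the mouse cursor.
; While InPlacement is true, Tick line-traces from the deprojected cursor on the Visibility channel and moves the actor to the hit point, snapped to a grid.
; Left mouse press clears InPlacement, ending the movement.
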(event `self.ReceiveBeginPlay`
  (bind _returnvalue (`GameplayStatics.GetPlayerController` 0))
  (`self.EnableInput` _returnvalue)
  (set `PlayerController.bShowMouseCursor` true _returnvalue))

(event `self.ReceiveTick`
  (params (DeltaSeconds :type "Float (single-precision)"))
  (bind (_worldlocation _worlddirection) (`PlayerController.DeprojectMousePositionToWorld` (`GameplayStatics.GetPlayerController` 0)))
  (if (`self.InPlacement`)
    (bind (_outhit _returnvalue) (`KismetSystemLibrary.LineTraceSingle` _worldlocation (+ _worldlocation (* _worlddirection 10000.0)) "TraceTypeQuery1"))
    (if _returnvalue
      (`self.K2_SetActorLocation` (`KismetMathLibrary.Vector_SnappedToGrid` (`.ImpactPoint` (`GameplayStatics.BreakHitResult` _outhit)) 100.0)))))

(event `Key|LeftMouseButton`
  (params (Key :type "Key Structure"))
  (:`Pressed`
    (if (`self.InPlacement`)
      (set `self.InPlacement` false))))

(fn `UserConstructionScript`)